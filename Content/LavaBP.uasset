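; Lava hazard Blueprint that rises upward while its switch flag is on.
; Each Tick, it moves the Plane and the root of the referenced Collider up by the same fixed, unswept world offset, with no delta-time scaling or height limit.
; The BeginOverlap function sets that flag from its Begin argument; the actor's own overlap event is unused.
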(event `self.ReceiveTick`
  (params (DeltaSeconds :type "Float (single-precision)"))
  (if (`self.SwitchRecieving`)
    (`SceneComponent.K2_AddWorldOffset` (`self.Plane`) (0.0 0.0 0.65) false false)
    (`SceneComponent.K2_AddWorldOffset` (`Actor.RootComponent` (`self.collider`)) (0.0 0.0 0.65) false false)))

(fn `Begin Overlap`
  (params (Begin :type Boolean))
  (set `self.SwitchRecieving` Begin))

(fn `UserConstructionScript`)